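; Ice variant of the generic weapon: a flower held by the first-person player that freezes water with a beam.
; BeginPlay attaches it to the GripPoint socket, adds the weapon input mapping and creates a deactivated placeholder Niagara beam.
; Holding shoot activates the beam and runs a debug-drawn box trace along the camera's forward vector.
; After a short hold, hits freeze river segments or create ice platforms on water collision actors; release deactivates the beam.
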(event Custom|CustEv_CreateParticles
  ;[1 1 1] creates the particles
  (bind _returnvalue (Niagara|SpawnSystemAttached "/Game/z_Stuff/Nate_2-12-24/NiagSys_IceBeamPlaceholder.NiagSys_IceBeamPlaceholder" (Variables|/Game/FirstPerson/Blueprints/BP_FirstPersonCharacter.BP_FirstPersonCharacter_C|GetWeapon (Variables|Default|GetAs%20BP%20First%20Person%20Character)) "GripPoint" "0, 0, 0" "0, 0, 0" "KeepRelativeOffset" false))
  (Variables|Default|SetIceBeamVarOld _returnvalue))

(event Input|EnhancedActionEvents|EnhancedInputActionIA_ShootButFlower
  (params (ActionValue :type Boolean) (ElapsedSeconds :type Float%20%28double-precision%29) (TriggeredSeconds :type Float%20%28double-precision%29) (InputAction :type Input%20Action%20Object%20Reference :default "/Game/z_Stuff/Nate_2-12-24/IA_ShootButFlower.IA_ShootButFlower"))
  (bind _as_bp_first_person_character (Variables|Default|GetAs%20BP%20First%20Person%20Character))
  (bind _icebeamvarold (Variables|Default|GetIceBeamVarOld))
  (bind _firstpersoncamera (Variables|/Game/FirstPerson/Blueprints/BP_FirstPersonCharacter.BP_FirstPersonCharacter_C|GetFirstPersonCamera _as_bp_first_person_character))
  (bind _returnvalue (Transformation|GetWorldLocation _firstpersoncamera))
  ;[1 1 1] activates/deactivates the flower's "shooting"
  (:Ongoing
    (Utilities|IsValid (Variables|Default|GetIceBeamVarOld)
      (:Is%20Valid
        _)
      (:Is%20Not%20Valid
        (CallFunction|CustEvCreateParticles)))
    (Components|Activation|Activate _icebeamvarold false)
    ;[1 1 1] Launces invisible hitscan box in direction player is facing. If it hits a RiverSegment after the ice beam has been active for a bit, it tells the river segment to activate the freeze event
    (bind _outhit (Class|KismetSystemLibrary|BoxTraceSingleforObjects _returnvalue (+ _returnvalue (* (Math|Vector|GetForwardVector _firstpersoncamera) (Math|Float|MakeLiteralFloat 5e+02))) "33.000000,33.000000,33.000000" (Transformation|GetActorRotation _as_bp_first_person_character) (Utilities|Array|MakeArray "ObjectTypeQuery1" "ObjectTypeQuery2" "ObjectTypeQuery1") false 0 "ForDuration" true))
    (if (>= ElapsedSeconds 1.2)
      (Utilities|FlowControl|Sequence
        (:then_0
          (bind _asbp_a_river_segment (Utilities|Casting|CastToBP_A_RiverSegment (.hitactor _outhit)))
          (Default|CustEvFreeze _asbp_a_river_segment))
        (:then_1
          (bind _asbp_a_water_collision_for_freeze (Utilities|Casting|CastToBP_A_WaterCollisionForFreeze (.hitactor _outhit)))
          (Default|CustEvMakeIcePlatform _asbp_a_water_collision_for_freeze (.location _outhit))))))
  (:Canceled
    (Components|Activation|Deactivate _icebeamvarold :!label _label))
  (:Completed
    (goto _label)))

(event EventBeginPlay
  ;[1 1 1] attatches flower to player character weapon slot
  (bind _asbp_first_person_character (Utilities|Casting|CastToBP_FirstPersonCharacter (Game|GetPlayerCharacter 0))
    (:then
      (bind _output_get (Variables|Default|SetAs%20BP%20First%20Person%20Character _asbp_first_person_character))
      (Variables|/Game/FirstPerson/Blueprints/BP_FirstPersonCharacter.BP_FirstPersonCharacter_C|SetWeapon _output_get self)
      (Transformation|AttachComponentToComponent (Variables|/Game/FirstPerson/Blueprints/BP_FirstPersonCharacter.BP_FirstPersonCharacter_C|GetFirstPersonMesh _output_get) "GripPoint" "SnapToTarget" "SnapToTarget" "SnapToTarget" true)
      ;[1 1 1] handles some of the controls having to do with using the "weapon"
      (bind _asplayer_controller (Utilities|Casting|CastToPlayerController (Pawn|GetController (Variables|Default|GetAs%20BP%20First%20Person%20Character))))
      (Utilities|IsValid (PlayerController|LocalPlayerSubsystems|GetEnhancedInputLocalPlayerSubsystem _asplayer_controller)
        (:Is%20Valid
          (Input|AddMappingContext (PlayerController|LocalPlayerSubsystems|GetEnhancedInputLocalPlayerSubsystem _asplayer_controller) "/Game/FirstPerson/Input/IMC_Weapons.IMC_Weapons" 1 "(bIgnoreAllPressedKeysUntilRelease=True,bForceImmediately=False,bNotifyUserSettings=False)")
          ;[1 1 1] creates and de-activates the particles
          (CallFunction|CustEvCreateParticles)
          (Components|Activation|Deactivate (Variables|Default|GetIceBeamVarOld)))))
    (:CastFailed
      (Development|PrintString "fuck"))))