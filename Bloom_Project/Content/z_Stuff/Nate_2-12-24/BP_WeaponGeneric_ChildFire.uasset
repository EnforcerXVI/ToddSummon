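; A flamethrower-style flower weapon that attaches to the first-person character's grip socket on BeginPlay and registers the weapons input mapping context.
; While the shoot input is held, it box-traces forward from the camera against world static and dynamic objects each tick and applies damage to what it hits.
; A math function, replacing an earlier timeline, grows the trace length with hold time up to a cap.
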(event Input|EnhancedActionEvents|EnhancedInputActionIA_ShootButFlower
  (params (ActionValue :type Boolean) (ElapsedSeconds :type Float%20%28double-precision%29) (TriggeredSeconds :type Float%20%28double-precision%29) (InputAction :type Input%20Action%20Object%20Reference :default "/Game/z_Stuff/Nate_2-12-24/IA_ShootButFlower.IA_ShootButFlower"))
  (bind _as_bp_first_person_character (Variables|Default|GetAs%20BP%20First%20Person%20Character))
  (bind _firstpersoncamera (Variables|/Game/FirstPerson/Blueprints/BP_FirstPersonCharacter.BP_FirstPersonCharacter_C|GetFirstPersonCamera _as_bp_first_person_character))
  (bind _returnvalue (Transformation|GetWorldLocation _firstpersoncamera))
  ;[0.2726 0 0.3177 0.597] Nate: Most of this code was done by Riley, was tweaked to work with modular parent-child system for flower items
  (:Ongoing
    (Variables|Default|SetFloat_FlammenLength (CallFunction|FuncFlameLengthMath ElapsedSeconds))
    (bind (_outhit _returnvalue_2) (Class|KismetSystemLibrary|BoxTraceSingleforObjects _returnvalue (+ _returnvalue (* (Math|Vector|GetForwardVector _firstpersoncamera) (Variables|Default|GetFloat_FlammenLength))) "15.000000,15.000000,15.000000" (Transformation|GetActorRotation _as_bp_first_person_character) (Utilities|Array|MakeArray "ObjectTypeQuery1" "ObjectTypeQuery2") false 0 "ForOneFrame" true))
    (if _returnvalue_2
      (Game|Damage|ApplyDamage (.HitActor (Collision|BreakHitResult _outhit)) 1.0 0 (Game|GetPlayerCharacter 0) "/Script/Engine.DamageType"))))

(event EventBeginPlay
  ;[1 1 1] attatches flower to player character
  (bind _asbp_first_person_character (Utilities|Casting|CastToBP_FirstPersonCharacter (Game|GetPlayerCharacter 0)))
  (bind _output_get (Variables|Default|SetAs%20BP%20First%20Person%20Character _asbp_first_person_character))
  (Variables|/Game/FirstPerson/Blueprints/BP_FirstPersonCharacter.BP_FirstPersonCharacter_C|SetWeapon _output_get self)
  (Transformation|AttachComponentToComponent (Variables|/Game/FirstPerson/Blueprints/BP_FirstPersonCharacter.BP_FirstPersonCharacter_C|GetFirstPersonMesh _output_get) "GripPoint" "SnapToTarget" "SnapToTarget" "SnapToTarget" true)
  ;[1 1 1] handles some of the controls having to do with using the "weapon"
  (bind _asplayer_controller (Utilities|Casting|CastToPlayerController (Pawn|GetController (Variables|Default|GetAs%20BP%20First%20Person%20Character))))
  (Utilities|IsValid (PlayerController|LocalPlayerSubsystems|GetEnhancedInputLocalPlayerSubsystem _asplayer_controller)
    (:Is%20Valid
      (Input|AddMappingContext (PlayerController|LocalPlayerSubsystems|GetEnhancedInputLocalPlayerSubsystem _asplayer_controller) "/Game/FirstPerson/Input/IMC_Weapons.IMC_Weapons" 1 "(bIgnoreAllPressedKeysUntilRelease=True,bForceImmediately=False,bNotifyUserSettings=False)"))))

(fn FuncFlameLengthMath
  (params (FloatParam :type Float%20%28double-precision%29))
  ;[1 1 1] This was originally a timeline but was reworked into a math function.
  ; Responsible for the length of the hitbox changing over time
  (if (>= FloatParam 1.5)
    (bind _output_get (LocalVariables|SetLocVar_Float 1e+03))
    (return _output_get)
    (else
      (return (* FloatParam 665.0)))))