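; Wind weapon Blueprint that clears BP_TempFog actors in front of the first-person player.
; On BeginPlay it registers as the player character's weapon, attaches to the mesh's GripPoint socket and adds the weapon input mapping context.
; While IA_ShootButFlower is ongoing, a debug-drawn box trace from the camera calls the kill-fog event on any fog actor it hits first.
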(event Input|EnhancedActionEvents|EnhancedInputActionIA_ShootButFlower
  (params (ActionValue :type Boolean) (ElapsedSeconds :type Float%20%28double-precision%29) (TriggeredSeconds :type Float%20%28double-precision%29) (InputAction :type Input%20Action%20Object%20Reference :default "/Game/z_Stuff/Nate_2-12-24/IA_ShootButFlower.IA_ShootButFlower"))
  (bind _first_personcharacter (Variables|Default|GetFirst%20PersonCharacter))
  (bind _firstpersoncamera (Variables|/Game/FirstPerson/Blueprints/BP_FirstPersonCharacter.BP_FirstPersonCharacter_C|GetFirstPersonCamera _first_personcharacter))
  (bind _returnvalue (Transformation|GetWorldLocation _firstpersoncamera))
  ;[0.2031 0 0] TODO: Finish documenting this
  (:Ongoing
    (bind _outhit (Class|KismetSystemLibrary|BoxTraceSingleforObjects _returnvalue (+ _returnvalue (* (Math|Vector|GetForwardVector _firstpersoncamera) (Math|Float|MakeLiteralFloat 5e+02))) "100.000000,100.000000,50.000000" (Transformation|GetActorRotation _first_personcharacter) (Utilities|Array|MakeArray "ObjectTypeQuery1" "ObjectTypeQuery2") false 0 "ForOneFrame" true))
    (bind _asbp_temp_fog (Utilities|Casting|CastToBP_TempFog (.hitactor _outhit)))
    (Default|CustEvKillFog _asbp_temp_fog)))

(event EventBeginPlay
  ;[0.2031 0 0] TODO: Finish documenting this
  (bind _asbp_first_person_character (Utilities|Casting|CastToBP_FirstPersonCharacter (Game|GetPlayerCharacter 0)))
  (bind _output_get (Variables|Default|SetFirst%20PersonCharacter _asbp_first_person_character))
  (Variables|/Game/FirstPerson/Blueprints/BP_FirstPersonCharacter.BP_FirstPersonCharacter_C|SetWeapon _output_get self)
  (Transformation|AttachComponentToComponent (Variables|/Game/FirstPerson/Blueprints/BP_FirstPersonCharacter.BP_FirstPersonCharacter_C|GetFirstPersonMesh _output_get) "GripPoint" "SnapToTarget" "SnapToTarget" "SnapToTarget" true)
  (bind _asplayer_controller (Utilities|Casting|CastToPlayerController (Pawn|GetController (Variables|Default|GetFirst%20PersonCharacter))))
  (Utilities|IsValid (PlayerController|LocalPlayerSubsystems|GetEnhancedInputLocalPlayerSubsystem _asplayer_controller)
    (:Is%20Valid
      (Input|AddMappingContext (PlayerController|LocalPlayerSubsystems|GetEnhancedInputLocalPlayerSubsystem _asplayer_controller) "/Game/FirstPerson/Input/IMC_Weapons.IMC_Weapons" 1 "(bIgnoreAllPressedKeysUntilRelease=True,bForceImmediately=False,bNotifyUserSettings=False)"))))

(event EventTick
  (params (DeltaSeconds :type Float%20%28single-precision%29)))